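; BP_DoorSocket is a socket that reacts when its Box trigger is overlapped, serving as the goal object's receiver for the exit.
; On overlap, with no check on the overlapping actor, it swaps the outline mesh to M_Frame and destroys the BP_GoalObject found by class lookup.
; It then turns the looked-up BP_ExitLight's point light green, plays DoorDing, and plays a second audio component after a short delay.
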(event `self.ReceiveBeginPlay`)

(event `self.Box.OnComponentBeginOverlap`
  (params (OverlappedComponent :type "PrimitiveComponent Object Reference") (OtherActor :type "Actor Object Reference") (OtherComp :type "PrimitiveComponent Object Reference") (OtherBodyIndex :type Integer) (bFromSweep :type Boolean) (SweepResult :type "HitResult Structure (by ref)"))
  ;[1 1 1] Door VFX and Sounds
  (`PrimitiveComponent.SetMaterial` (`self.SM_GoalObjectoutLine`) 0 "/Game/StarterContent/Props/Materials/M_Frame.M_Frame")
  (bind _returnvalue (`GameplayStatics.GetActorOfClass` "/Game/Gameplay_assesment/Blueprints/BP_GoalObject.BP_GoalObject_C"))
  (`self.K2_DestroyActor` _returnvalue)
  (bind _returnvalue_2 (`GameplayStatics.GetActorOfClass` "/Game/Gameplay_assesment/Blueprints/BP_ExitLight.BP_ExitLight_C"))
  (`LightComponent.SetLightColor` (`/Game/Gameplay_assesment/Blueprints/BP_ExitLight.PointLight` _returnvalue_2) (make `LinearColor` 0.0 100.0 0.0 1.0) true)
  (`AudioComponent.Play` (`self.DoorDing`) 0.0)
  (`KismetSystemLibrary.Delay` 0.5)
  (`AudioComponent.Play` (`self.Audio`) 0.0))

(fn `UserConstructionScript`)