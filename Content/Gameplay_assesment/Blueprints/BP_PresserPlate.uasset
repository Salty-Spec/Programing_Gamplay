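; BP_PresserPlate is a pressure plate that switches every BP_Button in the level on or off.
; BeginPlay caches all BP_Button actors.
; Box begin overlap plays CorrectPlate, sets each button Active and turns its RectLight and the plate's SpotLight green.
; End overlap stops CorrectPlate, clears Active and turns the lights red, with no filter on the overlapping actor in either event.
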(event `self.ReceiveBeginPlay`
  (bind _outactors (`GameplayStatics.GetAllActorsOfClass` "/Game/Gameplay_assesment/Blueprints/BP_Button.BP_Button_C")))

(event `self.Box.OnComponentBeginOverlap`
  (params (OverlappedComponent :type "PrimitiveComponent Object Reference") (OtherActor :type "Actor Object Reference") (OtherComp :type "PrimitiveComponent Object Reference") (OtherBodyIndex :type Integer) (bFromSweep :type Boolean) (SweepResult :type "HitResult Structure (by ref)"))
  (`AudioComponent.Play` (`self.Correct_Plate`) 0.0)
  (for _array_element (stale `self.ReceiveBeginPlay` _outactors)
    (`LightComponent.SetLightColor` (`/Game/Gameplay_assesment/Blueprints/BP_Button.RectLight` _array_element) (struct :`R` 0.019223 :`G` 0.682292 :`B` 0.029874 :`A` 1.0) true)
    (set `/Game/Gameplay_assesment/Blueprints/BP_Button.Active` true _array_element)
    (`LightComponent.SetLightColor` (`self.SpotLight`) (struct :`R` 0.019223 :`G` 0.682292 :`B` 0.029874 :`A` 1.0) true)))

(event `self.Box.OnComponentEndOverlap`
  (params (OverlappedComponent :type "PrimitiveComponent Object Reference") (OtherActor :type "Actor Object Reference") (OtherComp :type "PrimitiveComponent Object Reference") (OtherBodyIndex :type Integer))
  (`AudioComponent.Stop` (`self.Correct_Plate`))
  (for _array_element (stale `self.ReceiveBeginPlay` _outactors)
    (`LightComponent.SetLightColor` (`/Game/Gameplay_assesment/Blueprints/BP_Button.RectLight` _array_element) (struct :`R` 0.658375 :`B` 0.005605 :`A` 1.0) true)
    (set `/Game/Gameplay_assesment/Blueprints/BP_Button.Active` false _array_element)
    (`LightComponent.SetLightColor` (`self.SpotLight`) (struct :`R` 0.658375 :`B` 0.005605 :`A` 1.0) true)))

(fn `UserConstructionScript`)