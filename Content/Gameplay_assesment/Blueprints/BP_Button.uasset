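; BP_Button is an interactable puzzle button that activates linked BP_PUZZLEDOOR actors.
; On BeginPlay it caches every puzzle door in the level and enables mouse-over events.
; Interact, when the button is active and off cooldown, calls ActivateDoor on doors matching any of three DoorValues, with a short delay-based cooldown after a match.
; Hovering the pillar frame mesh shows a hand cursor, which is cleared when hover ends.
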(event `self.ReceiveBeginPlay`
  (bind _outactors (`GameplayStatics.GetAllActorsOfClass` "/Game/Gameplay_assesment/Blueprints/BP_PUZZLEDOOR.BP_PUZZLEDOOR_C"))
  (set `PlayerController.bEnableMouseOverEvents` true (`GameplayStatics.GetPlayerController` 0)))

(event `/Game/Gameplay_assesment/Blueprints/BPI_interact.Interact`
  (if (`self.Active`)
    (if (not (`self.OnCoolDown`))
      (for _array_element (stale `self.ReceiveBeginPlay` _outactors)
        (bind _doorvalue (`/Game/Gameplay_assesment/Blueprints/BP_PUZZLEDOOR.DoorValue` _array_element))
        (if (or (== _doorvalue (`self.DoorValue`)) (== _doorvalue (`self.DoorValue2`)) (== _doorvalue (`self.DoorValue3`)))
          (`/Game/Gameplay_assesment/Blueprints/BP_PUZZLEDOOR.ActivateDoor` _array_element)
          (set `self.OnCoolDown` true)
          (`KismetSystemLibrary.Delay` 2.0)
          (set `self.OnCoolDown` false))))))

(event `self.SM_PillarFrame.OnBeginCursorOver`
  (params (TouchedComponent :type "PrimitiveComponent Object Reference"))
  (set `PlayerController.CurrentMouseCursor` "Hand" (`GameplayStatics.GetPlayerController` 0)))

(event `self.SM_PillarFrame.OnEndCursorOver`
  (params (TouchedComponent :type "PrimitiveComponent Object Reference"))
  (set `PlayerController.CurrentMouseCursor` "None" (`GameplayStatics.GetPlayerController` 0)))

(fn `UserConstructionScript`)