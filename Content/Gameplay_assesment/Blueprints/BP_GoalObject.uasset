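; BP_GoalObject is a physics-driven goal object that can be thrown and sent back to a reset location, noted as the maze start.
; Its ThrowObject event overwrites the static mesh's linear velocity with the player camera's forward direction at a fixed speed.
; BeginPlay enables input from the first player controller, so pressing R teleports or moves the actor to ResetLocation without sweeping or clearing its velocity.
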(event `self.ReceiveBeginPlay`
  (`self.EnableInput` (`GameplayStatics.GetPlayerController` 0)))

(event `/Game/Gameplay_assesment/Blueprints/BPI_Grab.ThrowObject`
  ;[1 1 1] Throw Object
  (`PrimitiveComponent.SetPhysicsLinearVelocity` (`self.StaticMeshComponent`) (* (`KismetMathLibrary.GetForwardVector` (`PlayerCameraManager.GetCameraRotation` (`PlayerController.PlayerCameraManager` (`GameplayStatics.GetPlayerController` 0)))) 1000.0) false "None"))

(event `Key|R`
  (params (Key :type "Key Structure"))
  ;[1 1 1] Reset location to strart of maze
  (:`Pressed`
    (if true
      (`self.K2_SetActorLocation` self (`self.Reset Location`) false false))))

(fn `UserConstructionScript`)