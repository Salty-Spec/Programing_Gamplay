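; Teleport pad entrance that sends any actor overlapping its Box to the BP_TelePadEnd found in the level.
; On overlap it shows Sparks, adds an audio component and calls TeleportFXMessage on the end pad.
; After a short delay it moves the stored actor just above the end pad, without a sweep, and hides Sparks.
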(event `self.ReceiveBeginPlay`)

(event `self.Box.OnComponentBeginOverlap`
  (params (OverlappedComponent :type "PrimitiveComponent Object Reference") (OtherActor :type "Actor Object Reference") (OtherComp :type "PrimitiveComponent Object Reference") (OtherBodyIndex :type Integer) (bFromSweep :type Boolean) (SweepResult :type "HitResult Structure (by ref)"))
  (set `self.TeleportingActor` OtherActor)
  (bind _returnvalue (`GameplayStatics.GetActorOfClass` "/Game/Gameplay_assesment/Blueprints/BP_TelePadEnd.BP_TelePadEnd_C"))
  (`/Engine/EditorBlueprintResources/StandardMacros.IsValid` _returnvalue
    (:`Is Valid`
      (`SceneComponent.SetVisibility` (`self.Sparks`) true true)
      (`AddComponent|NODE_AddAudioComponent-0`)
      (message `/Game/Gameplay_assesment/Blueprints/BPI_Teleport.TeleportFX` _returnvalue)
      (`KismetSystemLibrary.Delay` 1.5)
      (`self.K2_SetActorLocation` (`self.TeleportingActor`) (+ (`self.K2_GetActorLocation` _returnvalue) (0.0 0.0 50.0)) false false)
      (`SceneComponent.SetVisibility` (`self.Sparks`) false true))))

(fn `UserConstructionScript`)